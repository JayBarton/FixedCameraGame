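; Inventory component that holds a fixed-size array of item slots and toggles its inventory window.
; On BeginPlay it sizes the array to the slot count.
; Adding writes non-stackable items into the first slot matching an empty struct, without checking for a full inventory; stackable items are not handled.
; Toggling creates or removes the window, centre-anchored on the player controller's HUD canvas, switching between UI-only and game-only input.
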(event EventBeginPlay
  (CallFunction|PrepareInventory))

(event EventTick
  (params (DeltaSeconds :type Float%20%28single-precision%29)))

(fn ToggleInventory
  (Variables|Default|GetInventoryWindow
    (:then
      (Widget|RemovefromParent (Variables|Default|GetInventoryWindow))
      (Variables|Default|SetInventoryWindow 0)
      (Input|SetInputModeGameOnly (Game|GetPlayerController 0)))
    (:else
      (bind _returnvalue (UserInterface|CreateWidget "/Game/Blueprints/InventoryTest/InventoryUI/InventoryWindow.InventoryWindow_C" 0 self))
      (bind _output_get (Variables|Default|SetInventoryWindow _returnvalue))
      (bind _asbp_player_controller (Utilities|Casting|CastToBP_PlayerController (Game|GetPlayerController 0)))
      (bind _returnvalue_2 (Class|CanvasPanel|AddChildtoCanvas (Variables|/Game/Blueprints/InventoryTest/InventoryUI/HUD.HUD_C|GetHUDCanvas (Variables|/Game/Blueprints/InventoryTest/BP_PlayerController.BP_PlayerController_C|GetHUDWidget _asbp_player_controller)) _output_get))
      (Class|CanvasPanelSlot|SetAutoSize _returnvalue_2 true)
      (Class|CanvasPanelSlot|SetAlignment _returnvalue_2 "(X=0.500000,Y=0.500000)")
      (Class|CanvasPanelSlot|SetAnchors _returnvalue_2 (Utilities|Struct|MakeAnchors "(X=0.500000,Y=0.500000)" "(X=0.500000,Y=0.500000)"))
      (Class|CanvasPanelSlot|SetPosition _returnvalue_2 (Variables|Default|GetPosition))
      (Input|SetInputModeUIOnly (Game|GetPlayerController 0) (Variables|Default|GetInventoryWindow) "LockAlways"))))

(fn AddtoInventory
  (params (ToAdd :type Slot%20Structure%20Structure))
  (if (not (.isstackable (.itemstructure ToAdd)))
    (CallFunction|CreateStack ToAdd)
    (return true)))

(fn PrepareInventory
  (Utilities|Array|Resize (Variables|Default|GetInventory) (Variables|Default|GetNumberOfSlots)))

(fn CreateStack
  (params (ToAdd :type Slot%20Structure%20Structure))
  (bind _inventory (Variables|Default|GetInventory))
  (Utilities|Array|SetArrayElem _inventory (Utilities|Array|FindItem _inventory (Utilities|Struct|MakeSlotStructure "(Name_2_C9C49E3541F8CBBC0D3694B1EAE31E4B=NSLOCTEXT(\"[F862D19846CB4EC750E9CA9EA7F94385]\", \"33E9B1AD43CD728667421CA2016E9644\", \"None\"),IsStackable_5_1EEFE8A140D83D8FDB3836BF68357E55=True,Thumbnail_8_59A28836472E7D324301ECBAF98AA7E8=None,Description_11_8437632840E91968A153B48E74712ABE=NSLOCTEXT(\"[F862D19846CB4EC750E9CA9EA7F94385]\", \"52F5C955443A098A4A6818BA4986324D\", \"None\"),IsConsumable_14_38CD78764A00D2664DA85BA5A223ED11=True,MaxStackSize_17_01ADC03D4E2E6B59BFE0A79FE4080F31=4,Durability_20_CA8BBCAB4B69D2F504D3C3952FF8D395=0.000000,Class_23_4993865141CEC6CA8A21A39759DFCE9A=None)")) ToAdd))