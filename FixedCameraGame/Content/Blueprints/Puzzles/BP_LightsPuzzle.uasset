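; BP_LightsPuzzle is the visual layer of a grid-based lights puzzle, displaying which lights are on and which one is selected.
; SetUp and Toggle both call SetLights, which swaps each TestLightProp in Boxes between on and off materials to match the boolean Grid.
; UpdateIndex moves a custom depth highlight from the previous box to the one at Index.
; The graph only reads Grid and Index, leaving puzzle logic outside this file.
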(event EventBeginPlay)

(event Collision|EventActorBeginOverlap
  (params (OtherActor :type Actor%20Object%20Reference)))

(event EventTick
  (params (DeltaSeconds :type Float%20%28single-precision%29)))

(event EventToggle
  (CallFunction|SetLights))

(event EventUpdateIndex
  (bind _astest_light_prop (Utilities|Casting|CastToTestLightProp (Utilities|Array|Get(acopy) (Variables|Default|Getboxes) (Variables|Default|GetPreviousIndex))))
  (Rendering|SetRenderCustomDepth (Variables|/Game/Blueprints/Puzzles/TestLightProp.TestLightProp_C|GetStaticMesh _astest_light_prop) false)
  (bind _astest_light_prop_2 (Utilities|Casting|CastToTestLightProp (Utilities|Array|Get(acopy) (Variables|Default|Getboxes) (Variables|Default|Getindex))))
  (Rendering|SetRenderCustomDepth (Variables|/Game/Blueprints/Puzzles/TestLightProp.TestLightProp_C|GetStaticMesh _astest_light_prop_2) true)
  (Variables|Default|SetPreviousIndex (Variables|Default|Getindex)))

(event EventSetUp
  (CallFunction|SetLights))

(fn ConstructionScript)

(fn SetLights
  (for (_array_element _array_index) (Variables|Default|Getgrid)
    (bind _astest_light_prop (Utilities|Casting|CastToTestLightProp (Utilities|Array|Get(acopy) (Variables|Default|Getboxes) _array_index)))
    (if _array_element
      (Rendering|Material|SetMaterial (Variables|/Game/Blueprints/Puzzles/TestLightProp.TestLightProp_C|GetStaticMesh _astest_light_prop) 0 "/Game/Materials/Powerbox/PBOn.PBOn")
      (else
        (Rendering|Material|SetMaterial (Variables|/Game/Blueprints/Puzzles/TestLightProp.TestLightProp_C|GetStaticMesh _astest_light_prop) 0 "/Game/Materials/Powerbox/PBOff.PBOff")))))