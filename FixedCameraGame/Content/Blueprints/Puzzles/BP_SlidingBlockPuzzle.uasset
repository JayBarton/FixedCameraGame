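; Sliding block puzzle Blueprint that extends a parent puzzle class with visual feedback on numbered TestProp blocks.
; On setup it writes each Grid value onto the matching block's WBP_TestNumber widget, mapping 1-based values to the Boxes array.
; Index updates move a custom depth highlight from the previous block to the one at the current Grid index.
; SpotLight visibility toggles remain as unconnected nodes.
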(event EventSetUp
  (|CallParentFunction)
  (CallFunction|SetText)
  (Variables|Default|SetCurrentElement (Utilities|Array|Get(acopy) (Variables|Default|Getgrid) (Variables|Default|Getindex)))
  (Class|FCSlidingBlockPuzzle|UpdateIndex))

(event EventUpdateIndex
  (bind _grid (Variables|Default|Getgrid))
  (bind _index (Variables|Default|Getindex))
  (bind _output (Utilities|Array|Get(acopy) _grid _index))
  (bind _returnvalue (- _output 1))
  (|CallParentFunction)
  (bind _astest_prop (Utilities|Casting|CastToTestProp (Utilities|Array|Get(acopy) (Variables|Default|Getboxes) (Variables|Default|GetCurrentElement))))
  (Rendering|SetRenderCustomDepth (Variables|/Game/Blueprints/Puzzles/TestProp.TestProp_C|GetStaticMesh _astest_prop) false)
  (if (> _output 0)
    (Variables|Default|SetCurrentElement _returnvalue)
    (bind _astest_prop_2 (Utilities|Casting|CastToTestProp (Utilities|Array|Get(acopy) (Variables|Default|Getboxes) _returnvalue)))
    (Rendering|SetRenderCustomDepth (Variables|/Game/Blueprints/Puzzles/TestProp.TestProp_C|GetStaticMesh _astest_prop_2) true)))

(fn ConstructionScript)

(fn SetText
  (for _array_element (Variables|Default|GetGrid)
    (bind _output_get (LocalVariables|SetCurrentBox _array_element))
    (if (>= _output_get 0)
      (bind _astest_prop (Utilities|Casting|CastToTestProp (Utilities|Array|Get(acopy) (Variables|Default|GetBoxes) (- (LocalVariables|GetCurrentBox) 1))))
      (bind _aswbp_test_number (Utilities|Casting|CastToWBP_TestNumber (UserInterface|GetUserWidgetObject (Variables|/Game/Blueprints/Puzzles/TestProp.TestProp_C|GetWidget _astest_prop))))
      (Rendering|Components|TextRender|SetText (Variables|/Game/Blueprints/Puzzles/WBP_TestNumber.WBP_TestNumber_C|GetNumber _aswbp_test_number) (Utilities|Text|ToText(Integer) (LocalVariables|GetCurrentBox))))))