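; Test sliding-number puzzle, controlled by possession, on a four-column grid stored as a flat integer array with a negative empty slot.
; Directional inputs move a wrapping selection index, and Interact slides that block into an adjacent gap, updating array and actor location.
; Enter calls SolvePuzzle when numbers are in order.
; SetUpBoxes spawns numbered TestProp blocks, but its only call here sits in unreachable code.
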(event EventPossessed
  (params (NewController :type Controller%20Object%20Reference)))

(event EventUnpossessed
  (params (OldController :type Controller%20Object%20Reference)))

(event Input|ActionEvents|InputActionUp
  (params (Key :type Key%20Structure :default "None"))
  (:Pressed
    (bind _output_get (Variables|Default|SetIndex (- (Variables|Default|GetIndex) 4)))
    (if (< _output_get 0)
      (Variables|Default|SetIndex (+ (Variables|Default|GetIndex) (Utilities|Array|Length (Variables|Default|GetGrid)))))
    (Development|PrintString (Utilities|String|ToString(Integer) (Variables|Default|GetIndex)))))

(event Input|ActionEvents|InputActionDown
  (params (Key :type Key%20Structure :default "None"))
  (bind _grid (Variables|Default|GetGrid))
  (bind _returnvalue (Utilities|Array|Length _grid))
  (:Pressed
    (bind _output_get (Variables|Default|SetIndex (+ (Variables|Default|GetIndex) 4)))
    (if (>= _output_get _returnvalue)
      (Variables|Default|SetIndex (- (Variables|Default|GetIndex) _returnvalue)))
    (Development|PrintString (Utilities|String|ToString(Integer) (Variables|Default|GetIndex)))))

(event Input|ActionEvents|InputActionInteract
  (params (Key :type Key%20Structure :default "None"))
  (:Pressed
    (bind _adjacentindex (CallFunction|FindAdjacent))
    (if (>= _adjacentindex 0)
      (CallFunction|MoveBlock _adjacentindex)
      (else
        (Development|PrintString "Nothing")))))

(event Input|ActionEvents|InputActionRight
  (params (Key :type Key%20Structure :default "None"))
  (:Pressed
    (bind _output_get (Variables|Default|SetIndex (+ (Variables|Default|GetIndex) 1)))
    (if (>= _output_get (Utilities|Array|Length (Variables|Default|GetGrid)))
      (Variables|Default|SetIndex 0))
    (Development|PrintString (Utilities|String|ToString(Integer) (Variables|Default|GetIndex)))))

(event Input|ActionEvents|InputActionLeft
  (params (Key :type Key%20Structure :default "None"))
  (:Pressed
    (bind _output_get (Variables|Default|SetIndex (- (Variables|Default|GetIndex) 1)))
    (if (< _output_get 0)
      (Variables|Default|SetIndex (- (Utilities|Array|Length (Variables|Default|GetGrid)) 1)))
    (Development|PrintString (Utilities|String|ToString(Integer) (Variables|Default|GetIndex)))))

(event Input|KeyboardEvents|Enter
  (params (Key :type Key%20Structure :default "None"))
  (:Pressed
    (CallFunction|CheckSolution)))

(fn ConstructionScript)

(fn FindAdjacent
  (Utilities|FlowControl|Sequence
    (:then_0
      (bind _output_get (LocalVariables|SetIndexToCheck (+ (Variables|Default|GetIndex) 1)))
      (if (> (Math|Integer|%(Integer) _output_get 4) 0)
        (if (< (Utilities|Array|Get(acopy) (Variables|Default|GetGrid) (LocalVariables|GetIndexToCheck)) 0)
          (return (LocalVariables|GetIndexToCheck)))))
    (:then_1
      (bind _output_get_2 (LocalVariables|SetIndexToCheck (- (Variables|Default|GetIndex) 1)))
      (if (and (< (Math|Integer|%(Integer) _output_get_2 4) 3) (>= _output_get_2 0))
        (if (< (Utilities|Array|Get(acopy) (Variables|Default|GetGrid) (LocalVariables|GetIndexToCheck)) 0)
          (return (LocalVariables|GetIndexToCheck)))))
    (:then_2
      (bind _output_get_3 (LocalVariables|SetIndexToCheck (+ (Variables|Default|GetIndex) 4)))
      (if (< _output_get_3 (Utilities|Array|Length (Variables|Default|GetGrid)))
        (if (< (Utilities|Array|Get(acopy) (Variables|Default|GetGrid) (LocalVariables|GetIndexToCheck)) 0)
          (return (LocalVariables|GetIndexToCheck)))))
    (:then_3
      (bind _output_get_4 (LocalVariables|SetIndexToCheck (- (Variables|Default|GetIndex) 4)))
      (if (>= _output_get_4 0)
        (if (< (Utilities|Array|Get(acopy) (Variables|Default|GetGrid) (LocalVariables|GetIndexToCheck)) 0)
          (return (LocalVariables|GetIndexToCheck)))))
    (:then_4
      (return -1))))

(fn MoveBlock
  (params (NewIndex :type Integer))
  (bind _startlocation (Variables|Default|GetStartLocation))
  (LocalVariables|SetBox (Utilities|Array|Get(acopy) (Variables|Default|GetBoxes) (- (Utilities|Array|Get(acopy) (Variables|Default|GetGrid) (Variables|Default|GetIndex)) 1)))
  (Utilities|Array|SetArrayElem (Variables|Default|GetGrid) NewIndex (Utilities|Array|Get(acopy) (Variables|Default|GetGrid) (Variables|Default|GetIndex)))
  (Transformation|SetActorLocation (LocalVariables|GetBox) (Math|Vector|MakeVector (- (.x _startlocation) (Math|Conversions|ToFloat(Integer) (* (/ NewIndex 4) 100))) (+ (.y _startlocation) (Math|Conversions|ToFloat(Integer) (* (Math|Integer|%(Integer) NewIndex 4) 100))) (.z _startlocation)) false false)
  (Utilities|Array|SetArrayElem (Variables|Default|GetGrid) (Variables|Default|GetIndex) -1))

(fn CheckSolution
  (for _index (range 0 (- (Utilities|Array|Length (Variables|Default|GetGrid)) 1))
    (if (== (Utilities|Array|Get(acopy) (Variables|Default|GetGrid) _index) (+ _index 1))
      (Math|Integer|IncrementInt (LocalVariables|GetSum))))
  (if (== (LocalVariables|GetSum) (- (Utilities|Array|Length (Variables|Default|GetGrid)) 1))
    (Class|FCPuzzlePawnBase|SolvePuzzle)
    (else
      (Development|PrintString "Nope"))))

(fn SetUpBoxes
  (bind _startlocation (Variables|Default|GetStartLocation))
  (for (_array_element _array_index) (Variables|Default|GetGrid)
    (bind _output_get (LocalVariables|SetCurrentElement _array_element))
    (if (>= _output_get 0)
      (bind _returnvalue (Game|SpawnActorfromClass "/Game/Blueprints/Puzzles/TestProp.TestProp_C" (Math|Transform|MakeTransform (Math|Vector|MakeVector (- (.x _startlocation) (Math|Conversions|ToFloat(Integer) (* (/ _array_index 4) 100))) (+ (.y _startlocation) (Math|Conversions|ToFloat(Integer) (* (Math|Integer|%(Integer) _array_index 4) 100))) (.z _startlocation))) "Undefined" 0 0))
      (Utilities|Array|SetArrayElem (Variables|Default|GetBoxes) (- (LocalVariables|GetCurrentElement) 1) _returnvalue)
      (bind _astest_prop (Utilities|Casting|CastToTestProp (Utilities|Array|Get(acopy) (Variables|Default|GetBoxes) (- (LocalVariables|GetCurrentElement) 1))))
      (bind _aswbp_test_number (Utilities|Casting|CastToWBP_TestNumber (UserInterface|GetUserWidgetObject (Variables|/Game/Blueprints/Puzzles/TestProp.TestProp_C|GetWidget _astest_prop))))
      (Rendering|Components|TextRender|SetText (Variables|/Game/Blueprints/Puzzles/WBP_TestNumber.WBP_TestNumber_C|GetNumber _aswbp_test_number) (Utilities|Text|ToText(Integer) (LocalVariables|GetCurrentElement))))))