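; BP_DotPuzzle is a puzzle actor that displays the on/off state of a grid of slot props.
; Slots holds rows, each pairing an array of prop references with a matching array of booleans.
; Its Toggle event walks every cell, casts the prop to BPSlotProp and swaps its mesh material to match the boolean.
; Toggle only updates visuals and never changes the stored states.
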(event EventBeginPlay)

(event Collision|EventActorBeginOverlap
  (params (OtherActor :type Actor%20Object%20Reference)))

(event EventTick
  (params (DeltaSeconds :type Float%20%28single-precision%29)))

(event EventToggle
  (for _array_element (Variables|Default|Getslots)
    (for _index (range 0 (- (Utilities|Array|Length (.prop (Utilities|Struct|BreakDotArray _array_element))) 1))
      (bind _asbpslot_prop (Utilities|Casting|CastToBPSlotProp (Utilities|Array|Get(acopy) (.prop (Utilities|Struct|BreakDotArray _array_element)) _index)))
      (if (Utilities|Array|Get(acopy) (.row (Utilities|Struct|BreakDotArray _array_element)) _index)
        (Rendering|Material|SetMaterial (Variables|/Game/Blueprints/Puzzles/BPSlotProp.BPSlotProp_C|GetStaticMesh _asbpslot_prop) 0 "/Engine/MapTemplates/Materials/BasicAsset03.BasicAsset03")
        (else
          (Rendering|Material|SetMaterial (Variables|/Game/Blueprints/Puzzles/BPSlotProp.BPSlotProp_C|GetStaticMesh _asbpslot_prop) 0 "/Engine/MapTemplates/Materials/BasicAsset01.BasicAsset01"))))))

(fn ConstructionScript)