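; Test interactable actor that jumps between a raised and a resting position in response to a switch.
; On BeginPlay it stores the static mesh's world location as the start position.
; The Switch event moves the whole actor straight up by a fixed offset when on and back to that stored position when off, instantly and without sweep.
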(event Switch(Switch)
  (params (isOn :type Boolean))
  (bind _startposition (Variables|Default|GetStartPosition))
  (if isOn
    (Transformation|SetActorLocation (Math|Vector|MakeVector (.x _startposition) (.y _startposition) (+ (.z _startposition) 2e+02)) false false)
    (else
      (Transformation|SetActorLocation (Variables|Default|GetStartPosition) false false))))

(event EventBeginPlay
  (Variables|Default|SetStartPosition (Transformation|GetWorldLocation (Variables|Default|GetStaticMesh))))

(event EventTick
  (params (DeltaSeconds :type Float%20%28single-precision%29)))

(fn ConstructionScript)