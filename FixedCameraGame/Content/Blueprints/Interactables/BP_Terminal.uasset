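; BP_Terminal is an interactable terminal that hosts a password screen for a puzzle lock.
; SendtoWidget casts the Widget component's user widget to WBP_TerminalScreen, stores it and passes in the terminal's Password.
; It binds the screen's Exit and Open events back to the actor, which call ExitPuzzle and OpenLock, both defined outside this graph.
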(event Custom|Exit%20Terminal
  (Class|FCPuzzleIneractable|ExitPuzzle))

(event Custom|Open%20Lock
  (Class|FCPuzzleIneractable|OpenLock))

(event EventBeginPlay)

(event Collision|EventActorBeginOverlap
  (params (OtherActor :type Actor%20Object%20Reference)))

(event EventTick
  (params (DeltaSeconds :type Float%20%28single-precision%29)))

(event EventSendtoWidget
  (bind _aswbp_terminal_screen (Utilities|Casting|CastToWBP_TerminalScreen (UserInterface|GetUserWidgetObject (Variables|Default|GetWidget))))
  (Variables|Default|SetTerminalScreen _aswbp_terminal_screen)
  (Variables|/Game/Blueprints/UI/Terminal/WBP_TerminalScreen.WBP_TerminalScreen_C|SetPassword (Variables|Default|GetTerminalScreen) (Variables|Default|Getpassword))
  (EventDispatchers|BindEventtoExit (Variables|Default|GetTerminalScreen) (delegate Custom|Exit%20Terminal))
  (EventDispatchers|BindEventtoOpen (Variables|Default|GetTerminalScreen) (delegate Custom|Open%20Lock)))

(fn ConstructionScript)