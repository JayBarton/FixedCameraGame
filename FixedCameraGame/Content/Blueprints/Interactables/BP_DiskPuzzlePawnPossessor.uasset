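; Disk puzzle interactable that manages the disk display actor representing the puzzle's locked, unlocked and completed states.
; BeginPlay spawns a starting display and binds to two locks: FCLock unlocking swaps it for a second display, while the Unlocker's linked lock unlocking teleports that display to an offset along world Y.
; After a short delay, an active puzzle without an FCLock swaps immediately, and an inactive one jumps straight to the completed layout.
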(event Custom|UnlockPuzzle
  (CallFunction|ChangeDisks))

(event Custom|CompletePuzzle
  (Transformation|SetActorTransform (Variables|Default|GetDiskEnd) (Variables|Default|GetEndTransform)))

(event EventBeginPlay
  (bind _returnvalue (Transformation|GetActorTransform))
  (bind _output_get (Variables|Default|SetStartTransform (Math|Transform|MakeTransform (Math|Vector|MakeVector (.x (.location _returnvalue)) (.y (.location _returnvalue)) 78.458138) (.rotation _returnvalue) (.scale _returnvalue))))
  (Variables|Default|SetEndTransform (Math|Transform|MakeTransform (Math|Vector|MakeVector (.x (.location _output_get)) (+ (.y (.location _output_get)) -4e+01) (.z (.location _output_get))) (.rotation _output_get) (.scale _output_get)))
  (bind _returnvalue_2 (Game|SpawnActorfromClass "/Game/Blueprints/Puzzles/BPDiskDisplayStart.BPDiskDisplayStart_C" (Variables|Default|GetStartTransform) "Undefined" 0 0))
  (Variables|Default|SetDiskStart _returnvalue_2)
  (EventDispatchers|BindEventtoUnlocked (Variables|Default|GetFCLock) (delegate Custom|UnlockPuzzle))
  (EventDispatchers|BindEventtoUnlocked (Variables|/Script/FixedCameraGame.FCUnlockComponent|GetlinkedLock (Variables|Default|GetUnlocker)) (delegate Custom|CompletePuzzle))
  (Utilities|FlowControl|Delay 0.2)
  (if (Variables|Default|Getactive)
    (Utilities|IsValid (Variables|Default|GetFCLock)
      (:Is%20Not%20Valid
        (CallFunction|ChangeDisks)))
    (else
      (CallFunction|ChangeDisks)
      (Transformation|SetActorTransform (Variables|Default|GetDiskEnd) (Variables|Default|GetEndTransform)))))

(fn ConstructionScript)

(fn ChangeDisks
  (Actor|DestroyActor (Variables|Default|GetDiskStart))
  (bind _returnvalue (Game|SpawnActorfromClass "/Game/Blueprints/Puzzles/BPDiskDisplayStart_2.BPDiskDisplayStart_2_C" (Variables|Default|GetStartTransform) "Undefined" 0 0))
  (Variables|Default|SetDiskEnd _returnvalue))