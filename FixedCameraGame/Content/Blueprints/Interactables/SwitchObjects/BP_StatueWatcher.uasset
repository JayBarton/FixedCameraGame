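; Puzzle watcher that checks four statues against an expected value sequence and unlocks a linked pickup when all match.
; It binds to each switch's end event and re-runs the ordered comparison whenever one finishes.
; On a match it presses its own FCSwitch, deactivates the switches and opens FCUnlock.
; FCSwitch's on and end events make the linked BP_CSVPickup interactable via its collision profile; the on event also propagates to every switch.
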(event Switchon(FCSwitch)
  (for _array_element (Variables|Default|GetSwitches)
    (Variables|/Script/FixedCameraGame.FCInteractable|Setactive _array_element false)
    (Default|CallSwitchon (Variables|/Script/FixedCameraGame.FCSwitchInteractable|GetSwitch _array_element)))
  (bind _asbp_csvpickup (Utilities|Casting|CastToBP_CSVPickup (Variables|/Script/FixedCameraGame.FCUnlockComponent|GetlinkedInteractable (Variables|Default|GetFCUnlock))))
  (Collision|SetCollisionProfileName (Variables|/Script/FixedCameraGame.FCInteractable|GetBoxComp _asbp_csvpickup) "InteractBox" true :!class /Script/Engine.PrimitiveComponent))

(event SwitchEnd(FCSwitch)
  (bind _asbp_csvpickup (Utilities|Casting|CastToBP_CSVPickup (Variables|/Script/FixedCameraGame.FCUnlockComponent|GetlinkedInteractable (Variables|Default|GetFCUnlock))))
  (Collision|SetCollisionProfileName (Variables|/Script/FixedCameraGame.FCInteractable|GetBoxComp _asbp_csvpickup) "InteractBox" true :!class /Script/Engine.PrimitiveComponent))

(event Custom|SwitchEnd_Event_0
  (CallFunction|CheckStatues))

(event EventBeginPlay
  (for _array_element (Variables|Default|GetSwitches)
    (EventDispatchers|AssignSwitchEnd (Variables|/Script/FixedCameraGame.FCSwitchInteractable|GetSwitch _array_element) (delegate Custom|SwitchEnd_Event_0))))

(fn ConstructionScript)

(fn CheckStatues
  (bind _fcunlock (Variables|Default|GetFCUnlock))
  (bind (_array_element _array_index) (Utilities|Array|ForEachLoopwithBreak (Variables|Default|GetStatues) :!label _label)
    (:LoopBody
      (if (== (Variables|/Game/Blueprints/Interactables/SwitchObjects/BP_Statue.BP_Statue_C|GetValue _array_element) (Utilities|Array|Get(acopy) (Variables|Default|GetValues) _array_index))
        (Math|Integer|IncrementInt (LocalVariables|GetSum))
        (else
          (goto _label Break))))
    (:Completed
      (if (== (LocalVariables|GetSum) 4)
        (Class|FCSwitchComponent|PressSwitch (Variables|Default|GetFCSwitch) true false false)
        (CallFunction|TurnOffStatues)
        (Class|FCUnlockComponent|OpenLock _fcunlock)
        (Utilities|Casting|CastToBP_CSVPickup (Variables|/Script/FixedCameraGame.FCUnlockComponent|GetlinkedInteractable _fcunlock))))))

(fn TurnOffStatues
  (for _array_element (Variables|Default|GetSwitches)
    (Variables|/Script/FixedCameraGame.FCInteractable|Setactive _array_element false)))