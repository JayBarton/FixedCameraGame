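; BP_EndSwitch is an interactable switch that, judging by its name, ends a level by taking over the player's movement.
; On BeginPlay it caches the BPFCPlayer reference after a short delay.
; Action snaps the player to the switch's location and rotation, sets a Complete flag and makes the player's capsule ignore GameTraceChannel4.
; Once Complete is set, Tick feeds constant forward movement input, walking the player onward automatically.
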(event EventBeginPlay
  (Utilities|FlowControl|Delay 0.2)
  (bind _returnvalue (Actor|GetActorOfClass "/Game/Blueprints/BPFCPlayer.BPFCPlayer_C"))
  (Variables|Default|SetPlayer _returnvalue))

(event EventTick
  (params (DeltaSeconds :type Float%20%28single-precision%29))
  (bind _player (Variables|Default|GetPlayer))
  (if (Variables|Default|Getcomplete)
    (Pawn|Input|AddMovementInput _player (Transformation|GetActorForwardVector _player) 1.0 false)))

(event EventAction
  (params (isOn :type Boolean))
  (bind _player (Variables|Default|GetPlayer))
  (Transformation|SetActorLocation _player (Transformation|GetActorLocation) false false)
  (Transformation|SetActorRotation _player (Transformation|GetActorRotation))
  (Variables|Default|Setcomplete true)
  (Collision|SetCollisionResponsetoChannel (Variables|/Script/Engine.Character|GetCapsuleComponent _player) "ECC_GameTraceChannel4" "ECR_Ignore"))

(fn ConstructionScript)