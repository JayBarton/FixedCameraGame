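; BP_Statue is a switchable puzzle statue that turns 90 degrees each time its Action event fires.
; A timeline lerps the actor's yaw from the stored rotation toward the next quarter turn.
; When the turn finishes, it saves the new rotation, advances a Value counter that wraps after four steps, and calls the MovedStatue dispatcher.
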(event EventBeginPlay
  (Variables|Default|SetCurrentRotation (Transformation|GetActorRotation)))

(event Collision|EventActorBeginOverlap
  (params (OtherActor :type Actor%20Object%20Reference)))

(event EventTick
  (params (DeltaSeconds :type Float%20%28single-precision%29)))

(event EventAction
  (params (isOn :type Boolean))
  (bind _open (Timeline|RotateTimeline PlayFromStart)
    (:Update
      (Transformation|SetActorRotation (Math|Rotator|Lerp(Rotator) (Variables|Default|GetCurrentRotation) (Math|Rotator|MakeRotator (.Roll (Math|Rotator|BreakRotator (Variables|Default|GetCurrentRotation))) (.Pitch (Math|Rotator|BreakRotator (Variables|Default|GetCurrentRotation))) (+ (.Yaw (Math|Rotator|BreakRotator (Variables|Default|GetCurrentRotation))) 9e+01)) _open)))
    (:Finished
      (Variables|Default|SetCurrentRotation (Transformation|GetActorRotation))
      (bind _result (Math|Integer|IncrementInt (Variables|Default|GetValue))
        (:%20%20
          (if (>= _result 4)
            (Variables|Default|SetValue 0))
          (Default|CallMovedStatue))))))

(fn ConstructionScript)