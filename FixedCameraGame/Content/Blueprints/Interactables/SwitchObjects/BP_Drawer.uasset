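; BP_Drawer is an interactable switch-object drawer that slides open when its Action event fires.
; BeginPlay caches the starting location and an end position offset along negative world Y, so the slide direction ignores actor rotation.
; Action plays a timeline from the start to lerp between them, with no closing path, while ToonState snaps the drawer straight to the open position.
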(event EventBeginPlay
  (bind _output_get (Variables|Default|SetStartPosition (Transformation|GetActorLocation)))
  (Variables|Default|SetEndPosition (Math|Vector|MakeVector (.x _output_get) (- (.y _output_get) 2e+01) (.z _output_get))))

(event EventToonState
  (Transformation|SetActorLocation (Variables|Default|GetEndPosition) false false))

(event EventAction
  (params (isOn :type Boolean))
  (bind _open (Timeline|MoveTimeline PlayFromStart)
    (:Update
      (Transformation|SetActorLocation (Math|Vector|Lerp(Vector) (Variables|Default|GetStartPosition) (Variables|Default|GetEndPosition) _open) false false))))

(fn ConstructionScript)