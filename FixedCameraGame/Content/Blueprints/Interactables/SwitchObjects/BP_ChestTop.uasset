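; Chest lid switch object that swings open when its Action event fires with IsOn true; switching off does nothing.
; Action plays a wooden chest sound and runs a timeline that lerps from the rotation cached at BeginPlay to EndRotation.
; ToonState snaps the lid straight to EndRotation, with no sound or animation.
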(event EventBeginPlay
  (Variables|Default|SetCurrentRotation (Transformation|GetActorRotation)))

(event EventToonState
  (Transformation|SetActorRotation (Variables|Default|GetEndRotation)))

(event EventAction
  (params (isOn :type Boolean))
  (if isOn
    (Audio|PlaySound2D "/Game/Audio/PuzzleSounds/573654__the_frisbee_of_peace__wooden-chest-open.573654__the_frisbee_of_peace__wooden-chest-open" 1.0 1.0 0.0 0 0)
    (bind _open (Timeline|RotateTimeline Play)
      (:Update
        (Transformation|SetActorRotation (Math|Rotator|Lerp(Rotator) (Variables|Default|GetCurrentRotation) (Variables|Default|GetEndRotation) _open))))))

(fn ConstructionScript)