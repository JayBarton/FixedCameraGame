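; BP_Lights is a switch-object Blueprint that controls the brightness of a group of spot lights.
; Its Action event loops over the Lights array and sets each SpotLightComponent to a high intensity when on, or a dimmer but non-zero intensity when off.
; A separate ToonState event sets every light to the same high intensity, with no on/off check.
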(event EventToonState
  (for _array_element (Variables|Default|GetLights)
    (Rendering|Components|Light|SetIntensity (Variables|/Script/Engine.SpotLight|GetSpotLightComponent _array_element) 2.5e+04)))

(event Collision|EventActorBeginOverlap
  (params (OtherActor :type Actor%20Object%20Reference)))

(event EventTick
  (params (DeltaSeconds :type Float%20%28single-precision%29)))

(event EventAction
  (params (isOn :type Boolean))
  (if isOn
    (for _array_element (Variables|Default|GetLights)
      (Rendering|Components|Light|SetIntensity (Variables|/Script/Engine.SpotLight|GetSpotLightComponent _array_element) 2.5e+04))
    (else
      (for _array_element_2 (Variables|Default|GetLights)
        (Rendering|Components|Light|SetIntensity (Variables|/Script/Engine.SpotLight|GetSpotLightComponent _array_element_2) 5e+03)))))

(event EventBeginPlay)

(fn ConstructionScript)