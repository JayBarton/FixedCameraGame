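; Switchable interactable that moves itself between its starting location and EndPosition when its Action event receives an on or off state.
; BeginPlay caches the start location, and Action plays separate on and off timelines from the start, their rate scaled by MovementDuration, to lerp the actor's world location without sweeping.
; ToonState skips the animation and snaps the actor straight to EndPosition.
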(event EventBeginPlay
  (Variables|Default|SetStartPosition (Transformation|GetActorLocation)))

(event EventAction
  (params (isOn :type Boolean))
  (Components|Timeline|SetPlayRate (Variables|Default|GetTurnOnTimeline) (/ 1.0 (Variables|Default|GetMovementDuration)))
  (if isOn
    (bind _alpha (Timeline|TurnOnTimeline PlayFromStart)
      (:Update
        (Transformation|SetActorLocation (Math|Vector|Lerp(Vector) (Variables|Default|GetStartPosition) (Variables|Default|GetEndPosition) _alpha) false false)))
    (else
      (bind _alpha_2 (Timeline|TurnOffTimeline PlayFromStart)
        (:Update
          (Transformation|SetActorLocation (Math|Vector|Lerp(Vector) (Variables|Default|GetStartPosition) (Variables|Default|GetEndPosition) _alpha_2) false false))))))

(event EventTick
  (params (DeltaSeconds :type Float%20%28single-precision%29)))

(event EventToonState
  (Transformation|SetActorLocation (Variables|Default|GetEndPosition) false false))

(fn ConstructionScript)