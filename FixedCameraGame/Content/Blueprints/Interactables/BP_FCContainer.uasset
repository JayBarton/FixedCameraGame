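; Interactable container that opens its inventory alongside the player's when its Action event fires.
; OpenContainer toggles the player's inventory in container mode, then creates a WBP_ContainerInventory widget bound to both inventories.
; The widget is stored on the container's Inventory and added to the player inventory window's canvas at a fixed position.
; Unconnected leftover nodes would move player items into empty container slots or add the widget to the viewport.
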(event EventAction
  (CallFunction|OpenContainer))

(fn ConstructionScript)

(fn OpenContainer
  (bind _inventory (Variables|Default|GetInventory))
  (bind _asbpfcplayer (Utilities|Casting|CastToBPFCPlayer (Game|GetPlayerCharacter 0)))
  (bind _output_get (LocalVariables|SetPlayer _asbpfcplayer))
  (Default|ToggleInventory _asbpfcplayer 1 (Variables|Default|GetInventory))
  (bind _returnvalue (UserInterface|CreateWidget "/Game/Blueprints/UI/WBP_ContainerInventory.WBP_ContainerInventory_C" 0 _inventory (Variables|/Script/FixedCameraGame.FCPlayer|GetInventory _output_get)))
  (Variables|/Script/FixedCameraGame.FCInventoryComponent|SetinventoryWindow _inventory _returnvalue)
  (bind _returnvalue_2 (Class|CanvasPanel|AddChildtoCanvas (Variables|/Game/Blueprints/UI/WBP_Inventory.WBP_Inventory_C|GetCanvas (Variables|/Game/Blueprints/BPFCPlayer.BPFCPlayer_C|GetInventoryWindow (LocalVariables|GetPlayer))) _returnvalue))
  (Class|CanvasPanelSlot|SetPosition _returnvalue_2 "(X=50.000000,Y=400.000000)"))