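; BP_Numpad is an interactable keypad lock puzzle that shows a password entry widget to the player.
; SendtoWidget creates WBP_NumPad with the actor's Password, shows the cursor, gives the widget focus in Game and UI input mode, and binds its Open and Exit events.
; Open calls OpenLock, then shares the Exit path, which calls ExitPuzzle and removes and clears the widget.
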(event Custom|OpenEvent
  (Class|FCPuzzleInteractable|OpenLock)
  (Class|FCPuzzleInteractable|ExitPuzzle)
  (Widget|RemovefromParent (Variables|Default|GetNumPadWidget))
  (Variables|Default|SetNumPadWidget 0))

(event Custom|ExitEvent
  (Class|FCPuzzleInteractable|ExitPuzzle)
  (Widget|RemovefromParent (Variables|Default|GetNumPadWidget))
  (Variables|Default|SetNumPadWidget 0))

(event EventBeginPlay)

(event Collision|EventActorBeginOverlap
  (params (OtherActor :type Actor%20Object%20Reference)))

(event EventTick
  (params (DeltaSeconds :type Float%20%28single-precision%29)))

(event EventSendtoWidget
  (bind _returnvalue (Game|GetPlayerController 0))
  (bind _returnvalue_2 (UserInterface|CreateWidget "/Game/Blueprints/UI/NumPad/WBP_NumPad.WBP_NumPad_C" 0 (Variables|Default|Getpassword)))
  (bind _output_get (Variables|Default|SetNumPadWidget _returnvalue_2))
  (UserInterface|Viewport|AddtoViewport _output_get 0)
  (Variables|/Script/Engine.PlayerController|SetbShowMouseCursor _returnvalue true)
  (Input|SetInputModeGameandUI _returnvalue _output_get "DoNotLock" true)
  (EventDispatchers|BindEventtoOpen _output_get (delegate Custom|OpenEvent))
  (EventDispatchers|BindEventtoExit _output_get (delegate Custom|ExitEvent))
  (Widget|SetKeyboardFocus (Variables|Default|GetNumPadWidget)))

(fn ConstructionScript)