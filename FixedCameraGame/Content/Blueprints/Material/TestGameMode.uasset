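; A test game mode that pulses a post-process material effect over time.
; SetUpPostProcess creates a dynamic instance of TestMaterial_Inst and sets it as a full-weight blendable in the Postprocess settings, though nothing in this file calls it.
; Tick drives the material's Alpha parameter with a squared sine of game time for a 0–1 pulse, then prints the value read back.
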(event EventBeginPlay)

(event EventTick
  (params (DeltaSeconds :type Float%20%28single-precision%29))
  (bind _material (Variables|Default|GetMaterial))
  (Rendering|Material|SetScalarParameterValue _material "Alpha" (Math|Float|Lerp 0.0 1.0 (Math|Float|Power (Math|Trig|Sin(Radians) (* 5 (Utilities|Time|GetTimeSeconds))) 2.0)) :!class /Script/Engine.MaterialInstanceDynamic)
  (bind _returnvalue (Rendering|Material|GetScalarParameterValue _material "Alpha" :!class /Script/Engine.MaterialInstanceDynamic))
  (Development|PrintString (Utilities|String|ToString(Float) _returnvalue)))

(fn ConstructionScript)

(fn SetUpPostProcess
  (bind _returnvalue (Rendering|Material|CreateDynamicMaterialInstance "/Game/Blueprints/Material/TestMaterial_Inst.TestMaterial_Inst" "None" "None" :!class /Script/Engine.KismetMaterialLibrary))
  (bind _output_get (Variables|Default|SetMaterial _returnvalue))
  (Variables|/Script/Engine.PostProcessVolume|SetSettings (Variables|Default|GetPostprocess) (Utilities|Struct|MakePostProcessSettings (Utilities|Struct|MakeWeightedBlendables (Utilities|Array|MakeArray (Utilities|Struct|MakeWeightedBlendable 1.0 _output_get))))))