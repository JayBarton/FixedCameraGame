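; Player controller that handles the inventory input and owns the inventory window.
; The OpenInventory press is forwarded to the BPFCPlayer character's ToggleInventory, separate from the controller's own ToggleInventory, which takes an inventory to display.
; That function creates or removes WBP_Inventory, switching input mode, mouse cursor and game pause along with it.
; On opening, it gives keyboard focus to the first inventory grid child.
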(event EventBeginPlay)

(event EventTick
  (params (DeltaSeconds :type Float%20%28single-precision%29)))

(event Input|ActionEvents|InputActionOpenInventory
  (params (Key :type Key%20Structure :default "None"))
  (:Pressed
    (bind _asbpfcplayer (Utilities|Casting|CastToBPFCPlayer (Game|GetPlayerCharacter 0)))
    (Default|ToggleInventory _asbpfcplayer)))

(fn ConstructionScript)

(fn ToggleInventory
  (params (Inventory :type FC%20Inventory%20Component%20Object%20Reference))
  (bind _returnvalue (Game|GetPlayerController 0))
  (bind _returnvalue_2 (Game|GetPlayerController 0))
  (Utilities|IsValid (Variables|Default|GetInventoryWindow)
    (:Is%20Valid
      (Widget|RemovefromParent (Variables|Default|GetInventoryWindow))
      (Variables|Default|SetInventoryWindow 0)
      (Input|SetInputModeGameOnly _returnvalue)
      (Variables|/Script/Engine.PlayerController|SetbShowMouseCursor _returnvalue false)
      (Game|SetGamePaused false))
    (:Is%20Not%20Valid
      (bind _returnvalue_3 (UserInterface|CreateWidget "/Game/Blueprints/UI/WBP_Inventory.WBP_Inventory_C" 0 Inventory 0 0 0))
      (Variables|Default|SetInventoryWindow _returnvalue_3)
      (UserInterface|Viewport|AddtoViewport _returnvalue_3 0)
      (Input|SetInputModeGameandUI _returnvalue_2 (Variables|Default|GetInventoryWindow) "DoNotLock" true)
      (Variables|/Script/Engine.PlayerController|SetbShowMouseCursor _returnvalue_2 true)
      (Game|SetGamePaused true)
      (Widget|SetKeyboardFocus (Class|PanelWidget|GetChildat (Variables|/Game/Blueprints/UI/WBP_Inventory.WBP_Inventory_C|GetInventoryGrid _returnvalue_3))))))