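; Prototype watcher actor that reacts to the death of an enemy spawned by a referenced EnemySpawn.
; Shortly after BeginPlay it binds to that enemy's killed event, then on death moves the enemy to its own transform and presses an FCSwitch with the player hidden.
; When the switch ends, it reveals the DroppedItem, enabling its collision and marking it active.
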(event SwitchEnd(FCSwitch)
  (bind _droppeditem (Variables|Default|GetDroppedItem))
  (Development|SetHiddeninGame (Variables|/Script/FixedCameraGame.FCInteractable|GetMeshComp _droppeditem) false false)
  (Collision|SetActorEnableCollision _droppeditem true)
  (Variables|/Script/FixedCameraGame.FCInteractable|Setactive _droppeditem true))

(event Custom|EnemyKilled_Event_0
  (bind _enemyspawn (Variables|Default|GetEnemySpawn))
  (bind _spawnedenemy (Variables|/Script/FixedCameraGame.FCEnemySpawn|GetspawnedEnemy _enemyspawn))
  (Transformation|SetActorLocation _spawnedenemy (Transformation|GetActorLocation) false false)
  (Transformation|SetActorRotation _spawnedenemy (Transformation|GetActorRotation))
  (Class|FCSwitchComponent|PressSwitch (Variables|Default|GetFCSwitch) false true))

(event EventBeginPlay
  (bind _enemyspawn (Variables|Default|GetEnemySpawn))
  (bind _spawnedenemy (Variables|/Script/FixedCameraGame.FCEnemySpawn|GetspawnedEnemy _enemyspawn))
  (Utilities|FlowControl|Delay 0.2)
  (Utilities|IsValid _spawnedenemy
    (:Is%20Valid
      (EventDispatchers|AssignEnemyKilled _spawnedenemy (delegate Custom|EnemyKilled_Event_0)))))

(fn ConstructionScript)