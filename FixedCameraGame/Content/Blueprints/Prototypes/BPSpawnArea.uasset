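; Prototype trigger area that makes a set of linked enemies play their spawn-in when the player walks into it.
; On the first BPFCPlayer overlap with the Box while active, it presses its FCSwitch with the animation pause, music and play-once settings, deactivates and calls PlaySpawnIn on each entry's SpawnedEnemy.
; It destroys itself immediately if the switch has no scene to play, otherwise when the switch signals its end.
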(event OnComponentBeginOverlap(Box)
  (params (OverlappedComponent :type Primitive%20Component%20Object%20Reference) (OtherActor :type Actor%20Object%20Reference) (OtherComp :type Primitive%20Component%20Object%20Reference) (OtherBodyIndex :type Integer) (bFromSweep :type Boolean) (SweepResult :type Hit%20Result%20Structure%20%28by%20ref%29))
  (if (Variables|Default|GetActive)
    (Utilities|Casting|CastToBPFCPlayer OtherActor)
    (Class|FCSwitchComponent|PressSwitch (Variables|Default|GetFCSwitch) (Variables|Default|GetPauseAnimation) false (Variables|Default|GetPlayMusic) (Variables|Default|GetPlayOnce))
    (Variables|Default|SetActive false)
    (for _array_element (Variables|Default|GetEnemies)
      (Class|FCEnemy|PlaySpawnin (Variables|/Script/FixedCameraGame.FCEnemySpawn|GetspawnedEnemy _array_element)))
    (if (not (Variables|/Script/FixedCameraGame.FCSwitchComponent|GetplayScene (Variables|Default|GetFCSwitch)))
      (Actor|DestroyActor))))

(event SwitchEnd(FCSwitch)
  (Actor|DestroyActor))

(event EventBeginPlay)

(event Collision|EventActorBeginOverlap
  (params (OtherActor :type Actor%20Object%20Reference)))

(event EventTick
  (params (DeltaSeconds :type Float%20%28single-precision%29)))

(fn ConstructionScript)