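; Player Blueprint that manages inventory, pickup, switch and save UI.
; The OpenInventory input, unless aiming, reloading or blocked, toggles the inventory or closes an open save menu; locked objects also open the inventory through Toggle.
; Menus and prompts pause the game and show the cursor, with pickup prompts adding a hit-test-invisible inventory display.
; Separate functions remove each prompt, though ClearSaveConfirm nulls SwitchButtons instead of SaveButtons.
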(event EventToggle
  (params (mode :type Integer) (lock :type FC%20Lock%20Component%20Object%20Reference) (containerInventory :type FC%20Inventory%20Component%20Object%20Reference))
  ;[1 1 1] Called when trying to open a locked object
  (CallFunction|ToggleInventory mode 0 lock))

(event EventCreatePickUpWidget
  (params (pickup :type Actor%20Object%20Reference))
  (bind _returnvalue (Game|GetPlayerController 0))
  (bind _asfcpickup (Utilities|Casting|CastToFCPickup pickup))
  (CallFunction|DisplayInventory)
  (bind _returnvalue_2 (UserInterface|CreateWidget "/Game/Blueprints/UI/Items/WBP_ItemButtons.WBP_ItemButtons_C" 0 _asfcpickup))
  (bind _output_get (Variables|Default|SetItemButtons _returnvalue_2))
  (UserInterface|Viewport|AddtoViewport _output_get 0)
  (Input|SetInputModeGameandUI _returnvalue _returnvalue_2 "DoNotLock" true)
  (Variables|/Script/Engine.PlayerController|SetbShowMouseCursor _returnvalue true)
  (Game|SetGamePaused true)
  (Input|DisableInput (Game|Player|GetPlayerPawn 0) _returnvalue))

(event EventDisplayInventoryWidget
  (CallFunction|DisplayInventory))

(event EventClearInventoryWidget
  (CallFunction|ClearInventoryWindow))

(event EventCreateSwitchWidget
  (params (switchInteractable :type FC%20Switch%20Interactable%20Object%20Reference))
  (bind _returnvalue (Game|GetPlayerController 0))
  (bind _returnvalue_2 (UserInterface|CreateWidget "/Game/Blueprints/UI/Switches/WBP_SwitchButtons.WBP_SwitchButtons_C" 0 switchInteractable))
  (Variables|Default|SetSwitchButtons _returnvalue_2)
  (UserInterface|Viewport|AddtoViewport _returnvalue_2 0)
  (Input|SetInputModeGameandUI _returnvalue 0 "DoNotLock" true)
  (Variables|/Script/Engine.PlayerController|SetbShowMouseCursor _returnvalue true)
  (Game|SetGamePaused true)
  (Input|DisableInput (Game|Player|GetPlayerPawn 0) _returnvalue))

(event EventCreateSaveWidget
  (params (token :type Integer) (playerStart :type Integer))
  (bind _returnvalue (Game|GetPlayerController 0))
  (bind _returnvalue_2 (UserInterface|CreateWidget "/Game/Blueprints/UI/SavingAndLoading/WBP_SaveButtons.WBP_SaveButtons_C" 0 token playerStart))
  (bind _output_get (Variables|Default|SetSaveButtons _returnvalue_2))
  (UserInterface|Viewport|AddtoViewport _output_get 0)
  (Input|SetInputModeGameandUI _returnvalue 0 "DoNotLock" true)
  (Variables|/Script/Engine.PlayerController|SetbShowMouseCursor _returnvalue true)
  (Game|SetGamePaused true)
  (Input|DisableInput (Game|Player|GetPlayerPawn 0) _returnvalue))

(event Input|ActionEvents|InputActionOpenInventory
  (params (Key :type Key%20Structure :default "None"))
  (:Pressed
    (bind _returnvalue (Class|FCPlayer|BlockingInput))
    (if (not (Math|Boolean|ORBoolean (Variables|Default|GetisAiming) (Variables|Default|GetisReloading) _returnvalue))
      ;[1 1 1] Not a fan of this
      (Utilities|IsValid (Variables|Default|GetSaveWindow)
        (:Is%20Valid
          (CallFunction|ToggleSaveMenu))
        (:Is%20Not%20Valid
          (CallFunction|ToggleInventory))))))

(fn ConstructionScript)

(fn ToggleInventory
  (params (Mode :type Integer) (ContainerInventory :type FC%20Inventory%20Component%20Object%20Reference) (Lock :type FC%20Lock%20Component%20Object%20Reference))
  (bind _returnvalue (Game|GetPlayerController 0))
  (bind _returnvalue_2 (Game|GetPlayerController 0))
  (Utilities|IsValid (Variables|Default|GetInventoryWindow)
    (:Is%20Valid
      (Widget|RemovefromParent (Variables|Default|GetInventoryWindow))
      (Variables|Default|SetInventoryWindow 0)
      (Variables|/Script/FixedCameraGame.FCInventoryComponent|SetinventoryWindow (Variables|Default|GetInventory) 0)
      (Input|SetInputModeGameOnly _returnvalue)
      (Variables|/Script/Engine.PlayerController|SetbShowMouseCursor _returnvalue false)
      (Game|SetGamePaused false)
      (Variables|Default|SetinInventory false))
    (:Is%20Not%20Valid
      (bind _returnvalue_3 (UserInterface|CreateWidget "/Game/Blueprints/UI/WBP_Inventory.WBP_Inventory_C" 0 (Variables|Default|GetInventory) Mode ContainerInventory Lock (and (not (Utilities|IsValid Lock)) (not (Utilities|IsValid ContainerInventory)))))
      (bind _output_get (Variables|Default|SetInventoryWindow _returnvalue_3))
      (Variables|/Script/FixedCameraGame.FCInventoryComponent|SetinventoryWindow (Variables|Default|GetInventory) _output_get)
      (UserInterface|Viewport|AddtoViewport _output_get 0)
      (Input|SetInputModeGameandUI _returnvalue_2 0 "DoNotLock" true)
      (Variables|/Script/Engine.PlayerController|SetbShowMouseCursor _returnvalue_2 true)
      (Game|SetGamePaused true)
      (bind _aswbp_inventory_slot (Utilities|Casting|CastToWBP_InventorySlot (Class|PanelWidget|GetChildat (Variables|/Game/Blueprints/UI/WBP_Inventory.WBP_Inventory_C|GetInventoryGrid (Variables|Default|GetInventoryWindow)))))
      (Widget|SetFocus (Variables|/Game/Blueprints/UI/WBP_InventorySlot.WBP_InventorySlot_C|GetSlotButton _aswbp_inventory_slot))
      (Widget|SetKeyboardFocus (Variables|/Game/Blueprints/UI/WBP_InventorySlot.WBP_InventorySlot_C|GetSlotButton _aswbp_inventory_slot))
      (Variables|Default|SetinInventory true))))

(fn ClearItemButtons
  (CallFunction|ClearInventoryWindow)
  (CallFunction|ClearItemWindow))

(fn UpdateSlot
  (params (SlotIndex :type Integer))
  (bind _aswbp_inventory_slot (Utilities|Casting|CastToWBP_InventorySlot (Class|PanelWidget|GetChildat (Variables|/Game/Blueprints/UI/WBP_Inventory.WBP_Inventory_C|GetInventoryGrid (Variables|Default|GetInventoryWindow)) SlotIndex)))
  (Default|SetUpSlot _aswbp_inventory_slot))

(fn ClearInventoryWindow
  (Utilities|IsValid (Variables|Default|GetInventoryWindow)
    (:Is%20Valid
      (Widget|RemovefromParent (Variables|Default|GetInventoryWindow))
      (Variables|Default|SetInventoryWindow 0))))

(fn ClearItemWindow
  (Widget|RemovefromParent (Variables|Default|GetItemButtons))
  (Variables|Default|SetItemButtons 0))

(fn DisplayInventory
  ;[1 1 1] Displays non-interactable player inventory
  (bind _returnvalue (UserInterface|CreateWidget "/Game/Blueprints/UI/WBP_Inventory.WBP_Inventory_C" 0 (Variables|Default|GetInventory) 0 0 0))
  (bind _output_get (Variables|Default|SetInventoryWindow _returnvalue))
  (Widget|SetVisibility _output_get "HitTestInvisible")
  (UserInterface|Viewport|AddtoViewport _output_get 0))

(fn ClearSwitchWindow
  (Widget|RemovefromParent (Variables|Default|GetSwitchButtons))
  (Variables|Default|SetSwitchButtons 0))

(fn ToggleSaveMenu
  (params (token :type Integer) (playerStart :type Integer))
  (bind _returnvalue (Game|GetPlayerController 0))
  (bind _returnvalue_2 (Game|GetPlayerController 0))
  (Utilities|IsValid (Variables|Default|GetSaveWindow)
    (:Is%20Valid
      (Widget|RemovefromParent (Variables|Default|GetSaveWindow))
      (Variables|Default|SetSaveWindow 0)
      (Input|SetInputModeGameOnly _returnvalue)
      (Variables|/Script/Engine.PlayerController|SetbShowMouseCursor _returnvalue false)
      (Game|SetGamePaused false)
      (Variables|Default|SetinInventory false))
    (:Is%20Not%20Valid
      (bind _returnvalue_3 (UserInterface|CreateWidget "/Game/Blueprints/UI/SavingAndLoading/WBP_SaveMenu.WBP_SaveMenu_C" 0 token playerStart))
      (bind _output_get (Variables|Default|SetSaveWindow _returnvalue_3))
      (UserInterface|Viewport|AddtoViewport _output_get 0)
      (Input|SetInputModeGameandUI _returnvalue_2 0 "DoNotLock" true)
      (Variables|/Script/Engine.PlayerController|SetbShowMouseCursor _returnvalue_2 true)
      (Game|SetGamePaused true)
      (Variables|Default|SetinInventory true))))

(fn ClearSaveConfirm
  (Widget|RemovefromParent (Variables|Default|GetSaveButtons))
  (Variables|Default|SetSwitchButtons 0))